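; BP_DungeonGameMode runs each timed dungeon round, from a one-second countdown to the return to the lobby.
; BeginPlay copies banked score, target and round from the game instance into the game state, which holds them during play.
; When time runs out or CheckAllPlayersDead finds nobody alive, FinishRound compares score to target.
; It writes advanced or reset run progress to the game instance, then ServerTravels to the lobby map.
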(event `self.ReceiveBeginPlay`
  (bind _asbp_dungeon_game_instance (cast `/Game/FPS/GameMode/BP_DungeonGameInstance` (`GameplayStatics.GetGameInstance`)))
  (bind _asbp_random_dungeon_game_state (cast `/RandomDungeon/score/BP_RandomDungeonGameState` (`GameplayStatics.GetGameState`)))
  (set `/RandomDungeon/score/BP_RandomDungeonGameState.BankedScore` (`/Game/FPS/GameMode/BP_DungeonGameInstance.RunBankedScore` _asbp_dungeon_game_instance) _asbp_random_dungeon_game_state)
  (set `/RandomDungeon/score/BP_RandomDungeonGameState.TargetScore` (`/Game/FPS/GameMode/BP_DungeonGameInstance.RunTargetScore` _asbp_dungeon_game_instance) _asbp_random_dungeon_game_state)
  (set `/RandomDungeon/score/BP_RandomDungeonGameState.CurrentRound` (`/Game/FPS/GameMode/BP_DungeonGameInstance.RunRound` _asbp_dungeon_game_instance) _asbp_random_dungeon_game_state)
  (bind _asbp_random_dungeon_game_state_2 (cast `/RandomDungeon/score/BP_RandomDungeonGameState` (`GameplayStatics.GetGameState`)))
  (set `/RandomDungeon/score/BP_RandomDungeonGameState.TimeRemaining` (`self.RoundDuration`) _asbp_random_dungeon_game_state_2)
  (bind _returnvalue (`KismetSystemLibrary.K2_SetTimerDelegate` (delegate `TickRoundTimer`) 1.0 true))
  (set `self.RoundTimerHandle` _returnvalue))

(event `TickRoundTimer`
  (bind _asbp_random_dungeon_game_state (cast `/RandomDungeon/score/BP_RandomDungeonGameState` (`GameplayStatics.GetGameState`)))
  (bind _output_get (set `/RandomDungeon/score/BP_RandomDungeonGameState.TimeRemaining` (- (`/RandomDungeon/score/BP_RandomDungeonGameState.TimeRemaining` _asbp_random_dungeon_game_state) 1) _asbp_random_dungeon_game_state))
  (if (<= _output_get 0)
    (`KismetSystemLibrary.K2_ClearAndInvalidateTimerHandle` (`self.RoundTimerHandle`))
    (`self.FinishRound`)))

(event `FinishRound`
  (bind _asbp_random_dungeon_game_state (cast `/RandomDungeon/score/BP_RandomDungeonGameState` (`GameplayStatics.GetGameState`)))
  (bind _asbp_dungeon_game_instance (cast `/Game/FPS/GameMode/BP_DungeonGameInstance` (`GameplayStatics.GetGameInstance`)))
  (if (>= (`/RandomDungeon/score/BP_RandomDungeonGameState.BankedScore` _asbp_random_dungeon_game_state) (`/RandomDungeon/score/BP_RandomDungeonGameState.TargetScore` _asbp_random_dungeon_game_state))
    (set `/Game/FPS/GameMode/BP_DungeonGameInstance.RunBankedScore` (`/RandomDungeon/score/BP_RandomDungeonGameState.BankedScore` _asbp_random_dungeon_game_state) _asbp_dungeon_game_instance)
    (set `/Game/FPS/GameMode/BP_DungeonGameInstance.RunTargetScore` (+ (`/RandomDungeon/score/BP_RandomDungeonGameState.TargetScore` _asbp_random_dungeon_game_state) 15) _asbp_dungeon_game_instance)
    (set `/Game/FPS/GameMode/BP_DungeonGameInstance.RunRound` (+ (`/RandomDungeon/score/BP_RandomDungeonGameState.CurrentRound` _asbp_random_dungeon_game_state) 1) _asbp_dungeon_game_instance)
    (else
      (set `/Game/FPS/GameMode/BP_DungeonGameInstance.RunBankedScore` 0 _asbp_dungeon_game_instance)
      (set `/Game/FPS/GameMode/BP_DungeonGameInstance.RunTargetScore` 15 _asbp_dungeon_game_instance)
      (set `/Game/FPS/GameMode/BP_DungeonGameInstance.RunRound` 1 _asbp_dungeon_game_instance)))
  (`KismetSystemLibrary.ExecuteConsoleCommand` "ServerTravel /Game/FPS/Maps/lobby" null))

(event `CheckAllPlayersDead`
  (set `self.AlivePlayerCount` 0)
  (bind _outactors (`GameplayStatics.GetAllActorsOfClass` "/Game/FPS/Character/BP_DungeonFPSCharacter.BP_DungeonFPSCharacter_C"))
  (for _array_element _outactors
    (bind _asbp_dungeon_fpscharacter (cast `/Game/FPS/Character/BP_DungeonFPSCharacter` _array_element))
    (if (> (`DungeonFPSCharacterBase.GetCurrentHealth` _asbp_dungeon_fpscharacter) 0.0)
      (set `self.AlivePlayerCount` (+ (`self.AlivePlayerCount`) 1))))
  (if (<= (`self.AlivePlayerCount`) 0)
    (`self.FinishRound`)))

(fn `UserConstructionScript`)

(fn `新函数`)