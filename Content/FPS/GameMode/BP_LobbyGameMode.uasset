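; Game mode for the lobby map of a dungeon run game.
; On BeginPlay it copies the banked score, target score and round from the dungeon game instance into the random dungeon game state and zeroes the remaining time.
; A StartGame event uses a ServerTravel console command to move to the game map.
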(event `self.ReceiveBeginPlay`
  (bind _asbp_dungeon_game_instance (cast `/Game/FPS/GameMode/BP_DungeonGameInstance` (`GameplayStatics.GetGameInstance`)))
  (bind _asbp_random_dungeon_game_state (cast `/RandomDungeon/score/BP_RandomDungeonGameState` (`GameplayStatics.GetGameState`)))
  (set `/RandomDungeon/score/BP_RandomDungeonGameState.BankedScore` (`/Game/FPS/GameMode/BP_DungeonGameInstance.RunBankedScore` _asbp_dungeon_game_instance) _asbp_random_dungeon_game_state)
  (set `/RandomDungeon/score/BP_RandomDungeonGameState.TargetScore` (`/Game/FPS/GameMode/BP_DungeonGameInstance.RunTargetScore` _asbp_dungeon_game_instance) _asbp_random_dungeon_game_state)
  (set `/RandomDungeon/score/BP_RandomDungeonGameState.CurrentRound` (`/Game/FPS/GameMode/BP_DungeonGameInstance.RunRound` _asbp_dungeon_game_instance) _asbp_random_dungeon_game_state)
  (set `/RandomDungeon/score/BP_RandomDungeonGameState.TimeRemaining` 0 _asbp_random_dungeon_game_state))

(event `StartGame`
  (`KismetSystemLibrary.ExecuteConsoleCommand` "ServerTravel /Game/FPS/Maps/game" null))

(fn `UserConstructionScript`)